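; Virtual production camera pawn (Virtual, Handheld or On Rails) driven by motion-controller tracking or keyboard/mouse, with zoom and aperture controls.
; Tick updates tracking, focus from line/sphere traces or a stored point, and camera-facing screens while player-possessed.
; Subsystem camera type Handheld buffers transforms to delay tracking and enables the media input feed with post-process blending.
; It also saves/restores camera settings, plays an optional sequence and builds editor labels.
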(event `self.ReceiveTick`
  (params (DeltaSeconds :type "Float (single-precision)"))
  ;[1 0 0] Tick
  (`|ExecutionSequence`
    (:`then_0`
      ;[1 0.76 0.09635] Trakcing delaying
      (`self.Process Tracking Delay`))
    (:`then_1`
      ;[0 0.4141 1] Adapting Aperture and Focus
      (`self.Process Focus`))
    (:`then_2`
      ;[0.429 1 0.02391] Processing screens
      (if (`.bSuccess` (cast `PlayerController` (`self.GetController`) :!pure true))
        (for _array_element (`self.Screens`)
          (bind (_screen _facecamera) (break `/ZOAN_VP/Blueprints/Camera/STR_ZVP_CameraScreenSettings` _array_element))
          (`self.SetActorHiddenInGame` _screen false)
          (bind (_enabled _roll _pitch _yaw) (break `/ZOAN_VP/Blueprints/Camera/STR_ZVP_FaceCameraSettings` _facecamera))
          (if _enabled
            (`SceneComponent.K2_SetWorldRotation` (`/ZOAN_VP/Blueprints/Screen/BP_ZVP_Screen.Plane Pivot` _screen) (`KismetMathLibrary.MakeRotator` (select `bool` _roll :`true` (.roll (`KismetMathLibrary.FindLookAtRotation` (`SceneComponent.K2_GetComponentLocation` (`self.CineCamera`)) (`SceneComponent.K2_GetComponentLocation` (`/ZOAN_VP/Blueprints/Screen/BP_ZVP_Screen.Plane Pivot` _screen))))) (select `bool` _pitch :`true` (.pitch (`KismetMathLibrary.FindLookAtRotation` (`SceneComponent.K2_GetComponentLocation` (`self.CineCamera`)) (`SceneComponent.K2_GetComponentLocation` (`/ZOAN_VP/Blueprints/Screen/BP_ZVP_Screen.Plane Pivot` _screen))))) (select `bool` _yaw :`true` (.yaw (`KismetMathLibrary.FindLookAtRotation` (`SceneComponent.K2_GetComponentLocation` (`self.CineCamera`)) (`SceneComponent.K2_GetComponentLocation` (`/ZOAN_VP/Blueprints/Screen/BP_ZVP_Screen.Plane Pivot` _screen)))))) false false)))))))

(event `InputAction|Reopen Camera Feed Action`
  (params (Key :type "Key Structure"))
  (bind _camera_input (`self.Get Camera Input`))
  ;[1 0.2856 0] Forcing all camera feed sources to reopen
  (:`Pressed`
    (bind _outactors (`GameplayStatics.GetAllActorsOfClass` "/ZOAN_VP/Blueprints/Screen/BP_ZVP_Screen.BP_ZVP_Screen_C"))
    (for _array_element _outactors
      (`MediaBundleActorBase.RequestCloseMediaSource` _array_element)
      (`MediaBundleActorBase.RequestOpenMediaSource` _array_element))
    ;[0.1393 0.432 1] Closing media player
    (`MediaPlayer.Close` (`self.Feed Media Player`))
    (if (`self.Should Render Camera Feed`) :!label _label
      ;[1 0.6094 0] Openning input camera feed
      (`/Engine/EditorBlueprintResources/StandardMacros.IsValid` _camera_input
        (:`Is Valid`
          (`MediaPlayer.OpenSource` (`self.Feed Media Player`) _camera_input))
        (:`Is Not Valid`
          (`KismetSystemLibrary.PrintString` "ERROR: Not a valid Media Input object!" true true (struct :`R` 1.0 :`A` 1.0) 10.0)))
      (else
        (`MediaPlayer.Close` (`self.Feed Media Player`))))))

(event `Setup Input Camera Feed`
  ;[0.9789 0.1905 1] Using post processing
  (`CameraComponent.SetPostProcessBlendWeight` (`self.CineCamera`) (select `bool` (`self.Should Render Camera Feed`) :`true` 1.0 :!type "Float (single-precision)"))
  (goto _label))

(event `Correct Camera Initial Position / Rotation`
  (bind (_returnvalue_roll _returnvalue_pitch _returnvalue_yaw) (`KismetMathLibrary.BreakRotator` (`KismetMathLibrary.NormalizedDeltaRotator` (`self.K2_GetActorRotation`) (`SceneComponent.K2_GetComponentRotation` (`self.MotionController`)))))
  (bind (_returnvalue_x _returnvalue_y) (`KismetMathLibrary.BreakVector` (- (`self.K2_GetActorLocation`) (`SceneComponent.K2_GetComponentLocation` (`self.MotionController`)))))
  ;[0 1 0.1854] Correcting initial camera position / rotation
  (`self.K2_AddActorWorldOffset` (`KismetMathLibrary.MakeVector` _returnvalue_x _returnvalue_y))
  (`self.K2_AddActorWorldRotation` (`KismetMathLibrary.MakeRotator` 0.0 0.0 _returnvalue_yaw)))

(event `Listen Subsystem`
  ;[0 0.1661 1] Listening to subsystem events
  (add `ZVP_Subsystem.OnVirtualCameraFocusTypeChanged` (subsystem `ZVP_Subsystem`) (delegate `On Virtual Camera Focus Type Changed`))
  (add `ZVP_Subsystem.OnCameraTypeChanged` (subsystem `ZVP_Subsystem`) (delegate `On Camera Type Changed`)))

(event `self.ReceiveUnpossessed`
  (params (OldController :type "Controller Object Reference"))
  ;[1 0 0.6453] Unpossessing camera and leaving screens
  (for _array_element (`self.Screens`)
    (bind (_screen _facecamera _exclusive) (break `/ZOAN_VP/Blueprints/Camera/STR_ZVP_CameraScreenSettings` _array_element))
    (`SceneComponent.K2_SetRelativeRotation` (`/ZOAN_VP/Blueprints/Screen/BP_ZVP_Screen.Plane Pivot` _screen) (struct :`Yaw` 180.0) false false)
    (if _exclusive
      (`self.SetActorHiddenInGame` _screen true))))

(event `On Virtual Camera Focus Type Changed`
  (params (VirtualCameraFocusType :type "EZVP_VirtualCameraFocusType Enum" :default "ZVP_None"))
  ;[0 0.1661 1] Listening to subsystem events
  (`self.Update Virtual Camera Focus Type`))

(event `On Camera Type Changed`
  (params (CameraType :type "EZVP_CameraType Enum" :default "ZVP_Virtual"))
  ;[0 0.1661 1] Listening to subsystem events
  (`self.Setup Input Camera Feed`))

(event `Get Fixed Focus Actor`
  ;[0.9922 0 1] Searching for fixed focus actor
  (bind _returnvalue (`GameplayStatics.GetActorOfClass` "/ZOAN_VP/Blueprints/Camera/BP_ZVP_FixedFocus.BP_ZVP_FixedFocus_C"))
  (`/Engine/EditorBlueprintResources/StandardMacros.IsValid` _returnvalue
    (:`Is Valid`
      (bind _output_get (set `self.Fixed Focus Actor` _returnvalue))
      (set `self.Tracked Focus Point Location` (`self.K2_GetActorLocation` _output_get)))))

(event `Update Camera Offset`
  ;[1 0.1172 0] Setting virtual camera offset
  (`SceneComponent.K2_SetRelativeTransform` (`self.TrackedCameraSlot`) (`self.Tracker Offset`) false false))

(event `Save Camera Settings`
  ;[0.05469 0 1] Camera saving / restoring settings
  (`|ExecutionSequence`
    (:`then_0`
      (set `self.Restore Transform` (`self.GetTransform`)))
    (:`then_1`
      (set `self.Restore Focal Length` (`CineCameraComponent.CurrentFocalLength` (`self.CineCamera`))))
    (:`then_2`
      (set `self.Restore Aperture` (`CineCameraComponent.CurrentAperture` (`self.CineCamera`))))))

(event `self.ReceiveBeginPlay`
  (bind (_camera_animation_levelsequence _camera_animation_loop) (break `/ZOAN_VP/Blueprints/Camera/STR_ZVP_CameraAnimation` (`self.Camera Animation`)))
  ;[1 0 0] Begin Play
  ;[0 1 0.1464] Initial Setup
  (`self.Listen Subsystem`)
  (`self.Setup Input Camera Feed`)
  (`self.Get Fixed Focus Actor`)
  ;[0 0.3672 1] Saving camera
  (`self.Save Camera Settings`)
  (`self.Update Camera Offset`)
  ;[0.4297 1 0] Setting up initial state
  (`self.Set Keyboard Mouse Controls` false)
  (`self.Update Tracking Channel`)
  ;[1 0.7701 0] Getting initial focal length
  (set `self.Desired Focal Length` (`CineCameraComponent.CurrentFocalLength` (`self.CineCamera`)))
  ;[1 0.09332 0.8697] Spawns camera animation if available
  (bind (_outactor _returnvalue) (`LevelSequencePlayer.CreateLevelSequencePlayer` _camera_animation_levelsequence (make `MovieSceneSequencePlaybackSettings` true (make `MovieSceneSequenceLoopCount` (select `bool` _camera_animation_loop :`true` -1)))))
  (set `self.Animation Player` _returnvalue))

(event `Restore Camera`
  ;[0.05469 0 1] Camera saving / restoring settings
  (`|ExecutionSequence`
    (:`then_1`
      (`self.K2_SetActorTransform` (`self.Restore Transform`)))
    (:`then_2`
      (set `CineCameraComponent.CurrentFocalLength` (`self.Restore Focal Length`) (`self.CineCamera`)))
    (:`then_3`
      (set `CineCameraComponent.CurrentAperture` (`self.Restore Aperture`) (`self.CineCamera`)))))

(event `Update Tracking Channel`
  ;[0.001644 0 1] Setting motion raw input channel
  (set `MotionControllerComponent.MotionSource` (`|GetEnumeratorName` (`self.Tracking Pad`)) (`self.MotionController`)))

(event `Set Movement Direction`
  (params (Direction :type "/ZOAN_VP/Blueprints/Camera/E_ZVP_MovementDirection Enum" :default "NewEnumerator0"))
  (bind (_returnvalue_roll _returnvalue_pitch _returnvalue_yaw) (`KismetMathLibrary.BreakRotator` (`SceneComponent.K2_GetComponentRotation` (`self.CineCamera`))))
  ;[1 0 0.6862] Setting movement direction
  (set `self.Movement Direction` (`KismetMathLibrary.GreaterGreater_VectorRotator` (`self.Get Direction Vector` Direction) (`KismetMathLibrary.MakeRotator` 0.0 0.0 _returnvalue_yaw))))

(event `self.ReceivePossessed`
  (params (NewController :type "Controller Object Reference"))
  (bind (_camera_animation_levelsequence _camera_animation_loop _camera_animation_restartonpossessed) (break `/ZOAN_VP/Blueprints/Camera/STR_ZVP_CameraAnimation` (`self.Camera Animation`)))
  ;[0.08067 1 0.6955] Possessed Event... Restart animaition if needed when camera being possessed
  (cast `PlayerController` NewController) ; Is it a player?
  (if _camera_animation_restartonpossessed
    (bind _animation_player (`self.Animation Player`)
      (:`then`
        (`MovieSceneSequencePlayer.JumpToFrame` _animation_player (make `FrameTime` (make `FrameNumber` 0))))
      (:`else`))))

(event `Set Control Enabled`
  (params (Value :type Boolean))
  ;[0 0.3672 1] Setting camera control
  (if Value
    (`Controller.Possess` (`GameplayStatics.GetPlayerController` 0) self)
    (`self.Update Virtual Camera Focus Type`)
    (else
      (set `self.Last Active Rotation` (`SceneComponent.RelativeRotation` (`self.MotionController`)))
      (`self.Restore Camera`))))

(event `Move Camera`
  (params (Value :type "Float (double-precision)"))
  ;[0 1 0.03906] Moving camera
  (`self.AddMovementInput` (`self.Movement Direction`) Value))

(event `Keyboard Camera Movement`
  (params (Direction :type "/ZOAN_VP/Blueprints/Camera/E_ZVP_MovementDirection Enum" :default "NewEnumerator0") (Value :type "Float (double-precision)"))
  (bind (_returnvalue_roll _returnvalue_pitch _returnvalue_yaw) (`KismetMathLibrary.BreakRotator` (`SceneComponent.K2_GetComponentRotation` (`self.CineCamera`))))
  ;[0 0.1797 1] Keyboard movement
  (`self.AddMovementInput` (`KismetMathLibrary.GreaterGreater_VectorRotator` (`self.Get Direction Vector` Direction) (`KismetMathLibrary.MakeRotator` 0.0 0.0 _returnvalue_yaw)) Value))

(event `Process Tracking Delay`
  (bind (_returnvalue_location _returnvalue_rotation) (`KismetMathLibrary.BreakTransform` (`SceneComponent.GetRelativeTransform` (`self.MotionController`))))
  (bind (_output_location _output_rotation) (`KismetMathLibrary.BreakTransform` (`|GetArrayItem` (`self.Delay Transforms`))))
  ;[0.2891 1 0] Delaying tracking
  (switch `EZVP_CameraType` (`ZVP_Subsystem.GetCameraType` (subsystem `ZVP_Subsystem`))
    (:`ZVP_Virtual`
      (`SceneComponent.K2_SetRelativeLocationAndRotation` (`self.DelayedMotionController`) _returnvalue_location _returnvalue_rotation false false :!label _label_2))
    (:`ZVP_Handheld`
      (`KismetArrayLibrary.Array_Set` (`self.Delay Transforms`) (`KismetMathLibrary.FTrunc` (* (`self.Time Delay`) (`KismetMathLibrary.MapRangeUnclamped` (`GameplayStatics.GetWorldDeltaSeconds`) 8.3333 16.666 120.0 60.0))) (`SceneComponent.GetRelativeTransform` (`self.MotionController`)) true)
      (`SceneComponent.K2_SetRelativeLocationAndRotation` (`self.DelayedMotionController`) _output_location _output_rotation false false)
      (`KismetArrayLibrary.Array_Remove` (`self.Delay Transforms`)))
    (:`ZVP_OnRails`
      (goto _label_2))))

(event `Process Focal Length Change`
  (params (`Delta Time` :type "Float (double-precision)"))
  ;[1 0.3182 0] Smooth focal length change (NOT IN USE) TODO: Fix this to use with action key bindings
  (set `CineCameraComponent.CurrentFocalLength` (`KismetMathLibrary.FInterpTo` (`CineCameraComponent.CurrentFocalLength` (`self.CineCamera`)) (`self.Desired Focal Length`) `Delta Time` (select `bool` (`self.Smooth Focal Length Change`) :`true` (`self.Focal Length Interp Speed`))) (`self.CineCamera`))
  (`KismetSystemLibrary.PrintString` (`KismetStringLibrary.Conv_DoubleToString` (`CineCameraComponent.CurrentFocalLength` (`self.CineCamera`)))))

(event `Set Focal Length`
  (params (Value :type "Float (double-precision)"))
  ;[0 1 0.3966] Setting focal length and camera offset
  (bind _output_get (set `CineCameraComponent.CurrentFocalLength` Value (`self.CineCamera`)))
  (if (`self.Should Render Camera Feed`)
    (set `self.Focal Length Range` (`KismetMathLibrary.MakeVector2D` _output_get _output_get))))

(event `Set Offset`
  (params (Vector :type "Vector Structure"))
  ;[0 1 0.3966] Setting focal length and camera offset
  (`SceneComponent.K2_SetRelativeLocation` (`self.TrackedCameraSlot`) Vector false false))

(event `Change Zoom`
  (params (Value :type "Float (double-precision)"))
  (bind (_focal_length_range_x _focal_length_range_y) (`KismetMathLibrary.BreakVector2D` (`self.Focal Length Range`)))
  ;[0 0.6484 1] Changing Focal Length
  (set `CineCameraComponent.CurrentFocalLength` (`KismetMathLibrary.FClamp` (- (`CineCameraComponent.CurrentFocalLength` (`self.CineCamera`)) (* (* Value (`GameplayStatics.GetWorldDeltaSeconds`)) (`self.Zoom Speed`))) _focal_length_range_x _focal_length_range_y) (`self.CineCamera`)))

(event `Update Virtual Camera Focus Type`
  ;[1 0.4029 0] Updating virtual focus type
  (setmembers `CameraFocusSettings` :`StructRef` (`CineCameraComponent.FocusSettings` (`self.CineCamera`)) :`FocusMethod` "Manual"))

(event `Automatic Process Aperture`
  (bind (_focal_length_range_x _focal_length_range_y) (`KismetMathLibrary.BreakVector2D` (`self.Focal Length Range`)))
  ;[1 0.4922 0] Automatic aperture process
  (set `CineCameraComponent.CurrentAperture` (`KismetMathLibrary.MapRangeClamped` (`CameraComponent.FieldOfView` (`self.CineCamera`)) _focal_length_range_x _focal_length_range_y 22.0 1.4) (`self.CineCamera`)))

(event `Change Aperture`
  (params (Value :type "Float (double-precision)"))
  (bind (_aperture_range_x _aperture_range_y) (`KismetMathLibrary.BreakVector2D` (`self.Aperture Range`)))
  (bind _currentaperture (`CineCameraComponent.CurrentAperture` (`self.CineCamera`)))
  ;[0.5289 1 0] Changing aperture
  (`KismetSystemLibrary.PrintString` (`KismetStringLibrary.Conv_DoubleToString` _currentaperture))
  (set `CineCameraComponent.CurrentAperture` (`KismetMathLibrary.FClamp` (+ _currentaperture (* (* Value (`GameplayStatics.GetWorldDeltaSeconds`)) (`self.Aperture Change Speed`))) _aperture_range_x _aperture_range_y) (`self.CineCamera`)))

(event `Set Aperture`
  (params (`New Aperture` :type "Float (double-precision)"))
  (bind (_aperture_range_x _aperture_range_y) (`KismetMathLibrary.BreakVector2D` (`self.Aperture Range`)))
  ;[0.8665 0.2257 1] Setting aperture
  (set `CineCameraComponent.CurrentAperture` (`KismetMathLibrary.FClamp` `New Aperture` _aperture_range_x _aperture_range_y) (`self.CineCamera`)))

(event `Process Focus`
  ;[1 0 0.5625] Focus process
  (switch `EZVP_VirtualCameraFocusType` (`ZVP_Subsystem.GetVirtualCameraFocusType` (subsystem `ZVP_Subsystem`))
    (:`ZVP_Automatic`
      (if (`self.Update Focus Point`)
        (`self.Process Focus Point Trace`)
        (else
          (`self.Process Focus Tracking` :!label _label_3))))
    (:`ZVP_Fixed`
      (bind _fixed_focus_actor (`self.Fixed Focus Actor`)
        (:`then`
          (set `self.Tracked Focus Point Location` (`self.K2_GetActorLocation` _fixed_focus_actor))
          (goto _label_3))
        (:`else`)))))

(event `Change Manual Focus Distance`
  (params (Value :type "Float (double-precision)"))
  (bind (_focal_length_range_x _focal_length_range_y) (`KismetMathLibrary.BreakVector2D` (`self.Focal Length Range`)))
  ;[0 1 0.6953] Setting manual focus
  (`CameraComponent.SetFieldOfView` (`self.CineCamera`) (`KismetMathLibrary.FClamp` (+ (`.ManualFocusDistance` (break `CameraFocusSettings` (`CineCameraComponent.FocusSettings` (`self.CineCamera`)))) (* (* Value (`GameplayStatics.GetWorldDeltaSeconds`)) (`self.Manual Focus Speed`))) _focal_length_range_x _focal_length_range_y)))

(event `Process Focus Point Trace`
  (bind (_focal_length_range_x _focal_length_range_y) (`KismetMathLibrary.BreakVector2D` (`self.Focal Length Range`)))
  (bind _returnvalue (`SceneComponent.K2_GetComponentLocation` (`self.CineCamera`)))
  (bind _returnvalue_2 (+ _returnvalue (* (`KismetMathLibrary.GetForwardVector` (`SceneComponent.K2_GetComponentRotation` (`self.CineCamera`))) (`self.Max Focus Ray Size`))))
  ;[1 0 0.5625] Focus process
  (switch `/ZOAN_VP/Blueprints/Camera/E_ZVP_FocusRayType` (`self.Focus Ray Type`)
    (:`NewEnumerator0`
      (bind _outhit (`KismetSystemLibrary.LineTraceSingle` _returnvalue _returnvalue_2 "TraceTypeQuery1"))
      (`self.Process Focus Hit Result` _outhit))
    (:`NewEnumerator1`
      (bind _outhit_2 (`KismetSystemLibrary.SphereTraceSingle` _returnvalue _returnvalue_2 (`KismetMathLibrary.MapRangeClamped` (`CameraComponent.FieldOfView` (`self.CineCamera`)) _focal_length_range_x _focal_length_range_y 0.125 2.0) "TraceTypeQuery1"))
      (`self.Process Focus Hit Result` _outhit_2))))

(event `Toggle Focus Method`
  ;[0 1 0.6953] Setting manual focus
  (`self.Set Auto Focus` (not (`self.Update Focus Point`))))

(event `Set Auto Focus`
  (params (`Use Auto Focus` :type Boolean))
  ;[0 1 0.6953] Setting manual focus
  (set `self.Update Focus Point` `Use Auto Focus`))

(event `Process Focus Tracking`
  (bind _tracked_focus_point_location (`self.Tracked Focus Point Location`))
  ;[1 0 0.5625] Focus process
  (`self.Set Manual Focus Distance` (`KismetMathLibrary.VSize` (- (`SceneComponent.K2_GetComponentLocation` (`self.CineCamera`)) _tracked_focus_point_location)))
  (`KismetSystemLibrary.DrawDebugSphere` _tracked_focus_point_location 2.0 6 (struct :`R` 1.0 :`A` 1.0) 0.0 0.05))

(event `Process Focus Hit Result`
  (params (Hit :type "HitResult Structure (by ref)"))
  (bind (_bblockinghit _binitialoverlap _time _distance _location) (`GameplayStatics.BreakHitResult` Hit))
  ;[1 0 0.5625] Focus process
  (set `self.Tracked Focus Point Location` _location)
  (`self.Set Manual Focus Distance` (select `bool` _bblockinghit :`false` (`self.Max Focus Ray Size`) :`true` _distance)))

(event `Set Manual Focus Distance`
  (params (Value :type "Float (double-precision)"))
  ;[1 0 0.5625] Focus process
  (setmembers `CameraFocusSettings` :`StructRef` (`CineCameraComponent.FocusSettings` (`self.CineCamera`)) :`ManualFocusDistance` Value))

(fn `Get Camera Group Name`
  (returns (`Group Name` :type Name))
  (return (select `EZVP_CameraGroup` (`self.Group`) :`ZVP_CamGroup1` "Group 1" :`ZVP_CamGroup2` "Group 2" :`ZVP_CamGroup3` "Group 3" :`ZVP_CamGroup4` "Group 4" :`ZVP_CamGroup5` "Group 5" :`ZVP_CamGroup6` "Group 6" :`ZVP_CamGroup7` "Group 7" :`ZVP_CamGroup8` "Group 8" :`ZVP_CamGroup9` "Group 9" :`ZVP_CamGroupAvatars` "Avatars" :!type "Name")))

(fn `Get Camera Input`
  (returns (`Camera Input` :type "MediaSource Object Reference"))
  (bind _returnvalue (`AssetRegistry.GetAssetByObjectPath` (`AssetRegistryHelpers.GetAssetRegistry`) (`KismetStringLibrary.Conv_StringToName` (`KismetSystemLibrary.Conv_SoftObjectReferenceToString` (`.CameraInputSoftPtr` (break `ZVP_SessionConfig` (`ZVP_Subsystem.GetSessionConfig` (subsystem `ZVP_Subsystem`)))))) false))
  (return (cast `MediaSource` (`AssetRegistryHelpers.GetAsset` _returnvalue) :!pure true)))

(fn `Get Camera Type`
  (returns (`Camera type` :type "EZVP_CameraType Enum"))
  (return (`self.Type`)))

(fn `Get Direction Vector`
  (params (Index :type "/ZOAN_VP/Blueprints/Camera/E_ZVP_MovementDirection Enum" :default "NewEnumerator0"))
  (returns (ReturnValue :type "Vector Structure"))
  (bind _returnvalue (select `/ZOAN_VP/Blueprints/Camera/E_ZVP_MovementDirection` Index :`NewEnumerator0` (1.0 0.0 0.0) :`NewEnumerator1` (-1.0 0.0 0.0) :`NewEnumerator2` (0.0 1.0 0.0) :`NewEnumerator3` (0.0 -1.0 0.0) :`NewEnumerator4` (0.0 0.0 1.0) :`NewEnumerator5` (0.0 0.0 -1.0) :!type "Vector Structure"))
  (return (select `bool` (and (`|EnumInequality` Index "NewEnumerator0") (`|EnumInequality` Index "NewEnumerator1")) :`false` _returnvalue :`true` (* _returnvalue 0.5))))

(fn `Set Focal Length Smooth Change`
  (params (Value :type Boolean))
  (set `self.Smooth Focal Length Change` Value))

(fn `Set Keyboard Mouse Controls`
  (params (Value :type Boolean))
  (bind _returnvalue (`self.GetController`))
  (bind (_returnvalue_roll _returnvalue_pitch _returnvalue_yaw) (`KismetMathLibrary.BreakRotator` (`SceneComponent.K2_GetComponentRotation` (`self.CineCamera`))))
  (`|ExecutionSequence`
    (:`then_0`
      ;[1 1 1] Setting current camera rotation to controller
      (`/Engine/EditorBlueprintResources/StandardMacros.IsValid` _returnvalue
        (:`Is Valid`
          (`Controller.SetControlRotation` _returnvalue (`KismetMathLibrary.MakeRotator` 0.0 (select `bool` (and (< _returnvalue_pitch -89.0) (> _returnvalue_pitch -91.0)) :`false` _returnvalue_pitch) _returnvalue_yaw)))))
    (:`then_1`
      ;[1 1 1] Using controller rotation
      (set `SpringArmComponent.bUsePawnControlRotation` (`local.Value`) (`self.SpringArm`)))
    (:`then_2`
      ;[1 1 1] Attaching to tracked or untracke components
      (set `SpringArmComponent.CameraRotationLagSpeed` (select `bool` (`local.Value`) :`true` (`self.Keyboard Rotation Lag`)) (`self.SpringArm`))
      (set `SpringArmComponent.bEnableCameraRotationLag` (`local.Value`) (`self.SpringArm`))
      (`SceneComponent.K2_AttachToComponent` (`self.SpringArm`) (select `bool` (or (`local.Value`) (`|EnumEquality` (`self.Type`) "ZVP_OnRails")) :`false` (`self.TrackedCameraSlot`) :`true` (`self.UntrackedCameraSlot`)) "None" "SnapToTarget" "SnapToTarget" "SnapToTarget" true))))

(fn `Should Render Camera Feed`
  (returns (Value :type Boolean))
  (return (`|EnumEquality` (`ZVP_Subsystem.GetCameraType` (subsystem `ZVP_Subsystem`)) "ZVP_Handheld")))

(fn `UserConstructionScript`
  (bind (_focal_length_range_x _focal_length_range_y) (`KismetMathLibrary.BreakVector2D` (`self.Focal Length Range`)))
  (bind (_aperture_range_x _aperture_range_y) (`KismetMathLibrary.BreakVector2D` (`self.Aperture Range`)))
  (bind (_returnvalue_x _returnvalue_y) (`KismetMathLibrary.BreakVector` (/ (+ (`TextRenderComponent.GetTextLocalSize` (`self.TitleText`)) (0.0 20.0 0.0)) 100.0)))
  (bind (_returnvalue_x_2 _returnvalue_y_2) (`KismetMathLibrary.BreakVector` (/ (+ (`TextRenderComponent.GetTextLocalSize` (`self.CameraTypeText`)) (0.0 20.0 0.0)) 100.0)))
  (`|ExecutionSequence`
    (:`then_0`
      ;[0.1041 0 1] Camera Title Text
      (`SceneComponent.K2_SetRelativeLocation` (`self.TitleSlot`) (0.0 0.0 110.0) false false)
      (`TextRenderComponent.K2_SetText` (`self.TitleText`) (`KismetTextLibrary.Conv_StringToText` (`self.Position Title`)))
      (`TextRenderComponent.K2_SetText` (`self.TitleTextMirror`) (`KismetTextLibrary.Conv_StringToText` (`self.Position Title`)))
      (`TextRenderComponent.SetTextRenderColor` (`self.TitleText`) (`self.Title Color`))
      (`TextRenderComponent.SetTextRenderColor` (`self.TitleTextMirror`) (`self.Title Color`))
      (`SceneComponent.SetRelativeScale3D` (`self.TitleBackground`) (`KismetMathLibrary.MakeVector` 0.01 _returnvalue_y 0.5)))
    (:`then_1`
      ;[1 0.4467 0] Camera Type Text
      (`TextRenderComponent.K2_SetText` (`self.CameraTypeText`) (`KismetTextLibrary.Conv_StringToText` (select `EZVP_CameraType` (`self.Type`) :`ZVP_Virtual` "Virtual" :`ZVP_Handheld` "Handheld" :`ZVP_OnRails` "On Rails")))
      (`TextRenderComponent.K2_SetText` (`self.CameraTypeTextMirror`) (`KismetTextLibrary.Conv_StringToText` (select `EZVP_CameraType` (`self.Type`) :`ZVP_Virtual` "Virtual" :`ZVP_Handheld` "Handheld" :`ZVP_OnRails` "On Rails")))
      (`TextRenderComponent.SetTextRenderColor` (`self.CameraTypeText`) (select `EZVP_CameraType` (`self.Type`) :`ZVP_Virtual` (`self.Virtual Type Color`) :`ZVP_Handheld` (`self.Handheld Type Color`) :`ZVP_OnRails` (`self.On Rails Type Color`)))
      (`TextRenderComponent.SetTextRenderColor` (`self.CameraTypeTextMirror`) (select `EZVP_CameraType` (`self.Type`) :`ZVP_Virtual` (`self.Virtual Type Color`) :`ZVP_Handheld` (`self.Handheld Type Color`) :`ZVP_OnRails` (`self.On Rails Type Color`)))
      (`SceneComponent.SetRelativeScale3D` (`self.CameraTypeBackground`) (`KismetMathLibrary.MakeVector` 0.01 _returnvalue_y_2 0.5)))
    (:`then_2`
      ;[1 0 0] Disabled Text
      (`SceneComponent.K2_SetRelativeLocation` (`self.DisabledTextSlot`) (0.0 0.0 170.0) false false)
      (`SceneComponent.SetVisibility` (`self.DisabledTextSlot`) (not (`self.Enabled`)) true))
    (:`then_3`
      ;[0 1 0.238] Group Text
      (if (`|EnumInequality` (`self.Group`) "ZVP_CamGroupNone")
        (`SceneComponent.SetVisibility` (`self.GroupSlot`) true true)
        (`SceneComponent.K2_AddRelativeLocation` (`self.TitleSlot`) (0.0 0.0 60.0) false false)
        (`SceneComponent.K2_AddRelativeLocation` (`self.DisabledTextSlot`) (0.0 0.0 60.0) false false)
        (`TextRenderComponent.K2_SetText` (`self.GroupText`) (`KismetTextLibrary.Conv_NameToText` (`self.Get Camera Group Name`)))
        (`TextRenderComponent.K2_SetText` (`self.GroupTextMirror`) (`KismetTextLibrary.Conv_NameToText` (`self.Get Camera Group Name`)))
        (else
          (`SceneComponent.SetVisibility` (`self.GroupSlot`) false true))))
    (:`then_4`
      ;[0.02431 0.4356 1] Setting Initial Values
      (set `self.Last Active Rotation` (`self.K2_GetActorRotation`))
      (`self.Set Aperture` (`self.Initial Aperture`)))
    (:`then_5`
      ;[0.4833 1 0] Camera Title Position
      (`SceneComponent.K2_SetRelativeTransform` (`self.UntrackedCameraSlot`) (`KismetMathLibrary.MakeTransform` (`KismetMathLibrary.MakeVector` 0.0 0.0 (select `EZVP_CameraType` (`self.Type`) :`ZVP_Virtual` 170.0 :`ZVP_Handheld` 170.0))) false false)
      (`SceneComponent.K2_SetRelativeTransform` (`self.CameraTitle`) (`KismetMathLibrary.MakeTransform` (`KismetMathLibrary.MakeVector` 0.0 0.0 (select `EZVP_CameraType` (`self.Type`) :`ZVP_Virtual` 170.0 :`ZVP_Handheld` 170.0))) false false))
    (:`then_6`
      ;[0.56 0.03367 1] Setting focal length range
      (setmembers `CameraLensSettings` :`StructRef` (`CineCameraComponent.LensSettings` (`self.CineCamera`)) :`MinFocalLength` _focal_length_range_x :`MaxFocalLength` _focal_length_range_y)
      ;[0 1 0.6238] Setting aperture range
      (setmembers `CameraLensSettings` :`StructRef` (`CineCameraComponent.LensSettings` (`self.CineCamera`)) :`MinFStop` _aperture_range_x :`MaxFStop` _aperture_range_y)
      ;[1 0 0.05077] Setting arrow enabled
      (`SceneComponent.SetVisibility` (`self.Arrow`) (`|EnumInequality` (`self.Type`) "ZVP_OnRails") true))))