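; Virtual production camera manager that switches between BP_ZVP_VirtualCamera actors and routes movement, look, zoom, aperture and focus input to the active one.
; It filters cameras by the ZVP subsystem's type and group, hides their exclusive screens, and rebuilds when either changes.
; On BeginPlay it starts media capture of the viewport to the session's configured output.
; Keyboard movement speed is interpolated and reduced at longer focal lengths.
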(event `Setup Screens`
  ;[1 0.1151 0.04209] Setting up screens
  (bind _outactors (`GameplayStatics.GetAllActorsOfClass` "/ZOAN_VP/Blueprints/Screen/BP_ZVP_Screen.BP_ZVP_Screen_C"))
  (for _array_element _outactors
    (`/ZOAN_VP/Blueprints/Screen/BP_ZVP_Screen.Adapt Camera Type` _array_element (`ZVP_Subsystem.GetCameraType` (subsystem `ZVP_Subsystem`)))))

(event `Setup Cameras`
  (bind _returnvalue (subsystem `ZVP_Subsystem`))
  ;[1 0.541 0] Setting up all cameras in the scene
  (`KismetArrayLibrary.Array_Clear` (`self.Cameras`))
  (`KismetArrayLibrary.Array_Clear` (`self.Active Camera Groups`))
  (bind _outactors (`GameplayStatics.GetAllActorsOfClass` "/ZOAN_VP/Blueprints/Camera/BP_ZVP_VirtualCamera.BP_ZVP_VirtualCamera_C"))
  (if (> (`KismetArrayLibrary.Array_Length` _outactors) 0)
    (for _array_element _outactors
      (if (`/ZOAN_VP/Blueprints/Camera/BP_ZVP_VirtualCamera.Enabled` _array_element)
        (bind _returnvalue_2 (`|EnumEquality` (`/ZOAN_VP/Blueprints/Camera/BP_ZVP_VirtualCamera.Get Camera Type` _array_element) (`ZVP_Subsystem.GetCameraType` _returnvalue)))
        (if _returnvalue_2
          ;[1 0.8095 0] Getting valid camera groups in the level
          (`KismetArrayLibrary.Array_AddUnique` (`self.Active Camera Groups`) (`/ZOAN_VP/Blueprints/Camera/BP_ZVP_VirtualCamera.Group` _array_element)))
        (if (and _returnvalue_2 (`|EnumEquality` (`/ZOAN_VP/Blueprints/Camera/BP_ZVP_VirtualCamera.Group` _array_element) (`ZVP_Subsystem.GetCameraGroup` _returnvalue)))
          (`KismetArrayLibrary.Array_Add` (`self.Cameras`) _array_element)
          ;[1 0.05046 0.9444] Hidding screens assigned to the camera if needed
          (for _array_element_2 (`/ZOAN_VP/Blueprints/Camera/BP_ZVP_VirtualCamera.Screens` _array_element)
            (bind (_screen _facecamera _exclusive) (break `/ZOAN_VP/Blueprints/Camera/STR_ZVP_CameraScreenSettings` _array_element_2))
            (`/Engine/EditorBlueprintResources/StandardMacros.IsValid` _screen
              (:`Is Valid`
                (if _exclusive
                  (`self.SetActorHiddenInGame` _screen true)))
              (:`Is Not Valid`
                (`KismetSystemLibrary.PrintString` "ERROR: Invalid Screen reference!" true true (struct :`R` 1.0 :`A` 1.0) 10.0)))))))
    (`self.Sort Camera Group Array`)
    (if (<= (`KismetArrayLibrary.Array_Length` (`self.Cameras`)) 0)
      (`KismetSystemLibrary.PrintString` "ERROR: No camera with desired Real Camera Type in the level!" true true (struct :`R` 1.0 :`A` 1.0) 10.0)
      (else
        (`self.Set Camera` 0)))
    (else
      (`KismetSystemLibrary.PrintString` "ERROR: No cameras in the level!" true true (struct :`R` 1.0 :`A` 1.0) 10.0))))

(event `InputAction|ToggleKeyboardMouseAction`
  (params (Key :type "Key Structure"))
  ;[0.1484 1 0] Toggling keyboard and mouse controls
  (:`Pressed`
    (set `self.Using Keyboard Mouse` (not (`self.Using Keyboard Mouse`)))
    (bind _outactors (`GameplayStatics.GetAllActorsOfClass` "/ZOAN_VP/Blueprints/Camera/BP_ZVP_VirtualCamera.BP_ZVP_VirtualCamera_C"))
    (for _array_element _outactors
      (`/ZOAN_VP/Blueprints/Camera/BP_ZVP_VirtualCamera.Set Keyboard Mouse Controls` _array_element (`self.Using Keyboard Mouse`)))))

(event `InputAxis|InputScaleAxis`
  (params (AxisValue :type "Float (single-precision)"))
  (bind (_keyboard_input_scale_range_x _keyboard_input_scale_range_y) (`KismetMathLibrary.BreakVector2D` (`self.Keyboard Input Scale Range`)))
  ;[1 0 0.3047] Changing keyboard input scale
  (set `self.Desired Keyboard Input Scale` (`KismetMathLibrary.FClamp` (+ (`self.Desired Keyboard Input Scale`) (* AxisValue (`self.Keyboard Input Scale Step`))) _keyboard_input_scale_range_x _keyboard_input_scale_range_y)))

(event `self.ReceiveBeginPlay`
  (bind _camera_output (`self.Get Camera Output`))
  (`|ExecutionSequence`
    (:`then_0`
      ;[1 0 0.04687] Creating media capture
      (`/Engine/EditorBlueprintResources/StandardMacros.IsValid` _camera_output
        (:`Is Valid`
          (bind _returnvalue (`MediaOutput.CreateMediaCapture` _camera_output))
          (set `self.Media Capture` _returnvalue))
        (:`Is Not Valid`
          (`KismetSystemLibrary.PrintString` "ERROR: No Media Output object!" true true (struct :`R` 1.0 :`A` 1.0) 10.0))))
    (:`then_1`
      ;[0.3359 1 0] Enabling input from Player Controller
      (`self.EnableInput` (`GameplayStatics.GetPlayerController` 0)))
    (:`then_2`
      ;[0 1 0.0625] Setting active scene viewport
      (`KismetSystemLibrary.Delay` 0.2)
      (bind _media_capture (`self.Media Capture`)
        (:`then`
          (`MediaCapture.CaptureActiveSceneViewport` :`self` _media_capture))
        (:`else`
          (`KismetSystemLibrary.PrintString` "ERROR: No Media Capture!" true true (struct :`R` 1.0 :`A` 1.0) 10.0))))
    (:`then_3`
      ;[1 0.2751 0] Setting up cameras
      (`self.Setup Cameras`))
    (:`then_4`
      ;[0 0.1328 1] Setting first camera
      (`self.Set Camera` 0))
    (:`then_5`
      ;[1 0.9609 0] Saving player controller reference for optimization
      (set `self.Player Controller` (`GameplayStatics.GetPlayerController` 0)))
    (:`then_6`
      ;[1 0 0.3984] Setting initial keyboard scale
      (bind _output_get (set `self.Current Keyboard Input Scale` (`self.Initial Keyboard Input Scale`)))
      (set `self.Desired Keyboard Input Scale` _output_get))
    (:`then_7`
      ;[1 0.4209 0] Listening to subsystem
      (add `ZVP_Subsystem.OnCameraTypeChanged` (subsystem `ZVP_Subsystem`) (delegate `On Camera Type Changed`))
      (add `ZVP_Subsystem.OnCameraGroupChanged` (subsystem `ZVP_Subsystem`) (delegate `On Camera Group Changed`)))
    (:`then_8`
      ;[0.4012 1 0] Inital setup of screens in the level
      (`self.Setup Screens`))))

(event `InputAction|MoveForwardAction`
  (params (Key :type "Key Structure"))
  ;[0.4062 0 1] Camera Movement
  (:`Pressed`
    (`self.Set Camera Movement Direction` "NewEnumerator0")))

(event `InputAction|MoveLeftAction`
  (params (Key :type "Key Structure"))
  ;[0.4062 0 1] Camera Movement
  (:`Pressed`
    (`self.Set Camera Movement Direction` "NewEnumerator3")))

(event `InputAction|MoveBackwardAction`
  (params (Key :type "Key Structure"))
  ;[0.4062 0 1] Camera Movement
  (:`Pressed`
    (`self.Set Camera Movement Direction` "NewEnumerator1")))

(event `InputAction|MoveUpAction`
  (params (Key :type "Key Structure"))
  ;[0.4062 0 1] Camera Movement
  (:`Pressed`
    (`self.Set Camera Movement Direction` "NewEnumerator4")))

(event `InputAxis|MouseXAxis`
  (params (AxisValue :type "Float (single-precision)"))
  ;[0.7109 1 0] Keyboard/Mouse inputs
  (bind _current_camera (`self.Current Camera`)
    (:`then`
      (`Pawn.AddControllerYawInput` _current_camera AxisValue))
    (:`else`)))

(event `InputAction|MoveRightAction`
  (params (Key :type "Key Structure"))
  ;[0.4062 0 1] Camera Movement
  (:`Pressed`
    (`self.Set Camera Movement Direction` "NewEnumerator2")))

(event `InputAction|MoveDownAction`
  (params (Key :type "Key Structure"))
  ;[0.4062 0 1] Camera Movement
  (:`Pressed`
    (`self.Set Camera Movement Direction` "NewEnumerator5")))

(event `Keyboard Change Zoom / Aperture`
  (params (Value :type "Float (double-precision)"))
  ;[0.7109 1 0] Keyboard/Mouse inputs
  (`self.Current Camera`
    (:`then`
      (if (`self.Secondary Action`)
        (`/ZOAN_VP/Blueprints/Camera/BP_ZVP_VirtualCamera.Change Aperture` (`self.Current Camera`) Value)
        (else
          (`/ZOAN_VP/Blueprints/Camera/BP_ZVP_VirtualCamera.Change Zoom` (`self.Current Camera`) Value))))
    (:`else`)))

(event `InputAxis|MouseYAxis`
  (params (AxisValue :type "Float (single-precision)"))
  ;[0.7109 1 0] Keyboard/Mouse inputs
  (bind _current_camera (`self.Current Camera`)
    (:`then`
      (`Pawn.AddControllerPitchInput` _current_camera AxisValue))
    (:`else`)))

(event `Set Camera Movement Direction`
  (params (Direction :type "/ZOAN_VP/Blueprints/Camera/E_ZVP_MovementDirection Enum" :default "NewEnumerator0"))
  ;[0.4062 0 1] Camera Movement
  (bind _current_camera (`self.Current Camera`)
    (:`then`
      (`/ZOAN_VP/Blueprints/Camera/BP_ZVP_VirtualCamera.Set Movement Direction` _current_camera Direction))
    (:`else`)))

(event `InputAxis|MovementAxis`
  (params (AxisValue :type "Float (single-precision)"))
  ;[0.4062 0 1] Camera Movement
  (bind _current_camera (`self.Current Camera`)
    (:`then`
      (`/ZOAN_VP/Blueprints/Camera/BP_ZVP_VirtualCamera.Move Camera` _current_camera AxisValue))
    (:`else`)))

(event `InputAxis|LeftMouseAxis`
  (params (AxisValue :type "Float (single-precision)"))
  ;[0.7109 1 0] Keyboard/Mouse inputs
  (`self.Keyboard Change Zoom / Aperture` AxisValue))

(event `InputAxis|KeyboardForwardAxis`
  (params (AxisValue :type "Float (single-precision)"))
  ;[0.7109 1 0] Keyboard/Mouse inputs
  (bind _current_camera (`self.Current Camera`)
    (:`then`
      (`/ZOAN_VP/Blueprints/Camera/BP_ZVP_VirtualCamera.Keyboard Camera Movement` _current_camera "NewEnumerator0" (* AxisValue (`self.Get Keyboard Mouse Scale`))))
    (:`else`)))

(event `InputAxis|RightMouseAxis`
  (params (AxisValue :type "Float (single-precision)"))
  ;[0.7109 1 0] Keyboard/Mouse inputs
  (`self.Keyboard Change Zoom / Aperture` AxisValue))

(event `InputAxis|KeyboardRightAxis`
  (params (AxisValue :type "Float (single-precision)"))
  ;[0.7109 1 0] Keyboard/Mouse inputs
  (bind _current_camera (`self.Current Camera`)
    (:`then`
      (`/ZOAN_VP/Blueprints/Camera/BP_ZVP_VirtualCamera.Keyboard Camera Movement` _current_camera "NewEnumerator2" (* AxisValue (`self.Get Keyboard Mouse Scale`))))
    (:`else`)))

(event `InputAction|NextCameraGroupAction`
  (params (Key :type "Key Structure"))
  ;[0 0.8309 1] Changing camera group
  (:`Pressed`
    (`self.Change Camera Group` "NewEnumerator0")))

(event `InputAction|ToggleFocusAction`
  (params (Key :type "Key Structure"))
  ;[0.5 1 0] Toggling focus method
  (:`Pressed`
    (bind _current_camera (`self.Current Camera`)
      (:`then`
        (`/ZOAN_VP/Blueprints/Camera/BP_ZVP_VirtualCamera.Toggle Focus Method` _current_camera))
      (:`else`))))

(event `InputAxis|KeyboardUpAxis`
  (params (AxisValue :type "Float (single-precision)"))
  ;[0.7109 1 0] Keyboard/Mouse inputs
  (bind _current_camera (`self.Current Camera`)
    (:`then`
      (`/ZOAN_VP/Blueprints/Camera/BP_ZVP_VirtualCamera.Keyboard Camera Movement` _current_camera "NewEnumerator4" (* AxisValue (`self.Get Keyboard Mouse Scale`))))
    (:`else`)))

(event `On Camera Type Changed`
  (params (CameraType :type "EZVP_CameraType Enum" :default "ZVP_Virtual"))
  ;[1 0.4209 0] Listening to subsystem
  (`self.Setup Cameras`)
  (`self.Setup Screens`))

(event `On Camera Group Changed`
  (params (CameraGroup :type "EZVP_CameraGroup Enum" :default "ZVP_CamGroupNone"))
  ;[1 0.4209 0] Listening to subsystem
  (`self.Setup Cameras`))

(event `InputAction|PreviousCameraGroupAction`
  (params (Key :type "Key Structure"))
  ;[0 0.8309 1] Changing camera group
  (:`Pressed`
    (`self.Change Camera Group` "NewEnumerator1")))

(event `self.ReceiveTick`
  (params (DeltaSeconds :type "Float (single-precision)"))
  ;[1 0 0] Tick
  (`self.Process Keyboard Input Scale` DeltaSeconds)
  (`self.Process Aperture`))

(event `Apply Aperture Change`
  (params (Value :type "Float (double-precision)"))
  ;[1 0 0.9609] Changing aperture
  (bind _current_camera (`self.Current Camera`)
    (:`then`
      (`/ZOAN_VP/Blueprints/Camera/BP_ZVP_VirtualCamera.Change Aperture` _current_camera Value))
    (:`else`)))

(event `InputAction|IncreaseApertureAction`
  (params (Key :type "Key Structure"))
  ;[1 0 0.9609] Changing aperture
  (:`Pressed`
    (set `self.Increase Aperture` true))
  (:`Released`
    (set `self.Increase Aperture` false)))

(event `Key|One`
  (params (Key :type "Key Structure"))
  ;[0 0.7656 1] Camera indexes
  (:`Pressed`
    (`self.Set Camera` 0)))

(event `Key|Six`
  (params (Key :type "Key Structure"))
  ;[0 0.7656 1] Camera indexes
  (:`Pressed`
    (`self.Set Camera` 5)))

(event `InputAxis|ZoomAxis`
  (params (AxisValue :type "Float (single-precision)"))
  ;[0.875 0 1] Zooming
  (bind _current_camera (`self.Current Camera`)
    (:`then`
      (`/ZOAN_VP/Blueprints/Camera/BP_ZVP_VirtualCamera.Change Zoom` _current_camera (* AxisValue (select `bool` (`self.Secondary Action`) :`false` 1.0 :`true` -1.0 :!type "Float (single-precision)"))))
    (:`else`)))

(event `InputAction|DecreaseApertureAction`
  (params (Key :type "Key Structure"))
  ;[1 0 0.9609] Changing aperture
  (:`Pressed`
    (set `self.Decrease Aperture` true))
  (:`Released`
    (set `self.Decrease Aperture` false)))

(event `Process Keyboard Input Scale`
  (params (DeltaTime :type "Float (double-precision)"))
  ;[0 1 0.6953] Processing keyboard input scale
  (bind _output_get (set `self.Current Keyboard Input Scale` (`KismetMathLibrary.FInterpTo` (`self.Current Keyboard Input Scale`) (`self.Desired Keyboard Input Scale`) DeltaTime (`self.Keyboard Input Scale Interp Speed`)))))

(event `Key|Two`
  (params (Key :type "Key Structure"))
  ;[0 0.7656 1] Camera indexes
  (:`Pressed`
    (`self.Set Camera` 1)))

(event `Key|Seven`
  (params (Key :type "Key Structure"))
  ;[0 0.7656 1] Camera indexes
  (:`Pressed`
    (`self.Set Camera` 6)))

(event `Key|Three`
  (params (Key :type "Key Structure"))
  ;[0 0.7656 1] Camera indexes
  (:`Pressed`
    (`self.Set Camera` 2)))

(event `Key|Eight`
  (params (Key :type "Key Structure"))
  ;[0 0.7656 1] Camera indexes
  (:`Pressed`
    (`self.Set Camera` 7)))

(event `Process Aperture`
  ;[1 0 0.9609] Changing aperture
  (if (`self.Secondary Action`)
    (`|ExecutionSequence`
      (:`then_0`
        (if (`self.Increase Aperture`)
          (`self.Apply Aperture Change` 1.0)))
      (:`then_1`
        (if (`self.Decrease Aperture`)
          (`self.Apply Aperture Change` -1.0))))))

(event `InputAction|SecondaryAction`
  (params (Key :type "Key Structure"))
  ;[0.875 0 1] Zooming
  (:`Pressed`
    (set `self.Secondary Action` true))
  (:`Released`
    (set `self.Secondary Action` false)))

(event `Key|Four`
  (params (Key :type "Key Structure"))
  ;[0 0.7656 1] Camera indexes
  (:`Pressed`
    (`self.Set Camera` 3)))

(event `Key|Nine`
  (params (Key :type "Key Structure"))
  ;[0 0.7656 1] Camera indexes
  (:`Pressed`
    (`self.Set Camera` 8)))

(event `Key|Five`
  (params (Key :type "Key Structure"))
  ;[0 0.7656 1] Camera indexes
  (:`Pressed`
    (`self.Set Camera` 4)))

(event `Key|Zero`
  (params (Key :type "Key Structure"))
  ;[0 0.7656 1] Camera indexes
  (:`Pressed`
    (`self.Set Camera` 9)))

(event `InputAction|NextCameraAction`
  (params (Key :type "Key Structure"))
  ;[0.4335 1 0] Selecting next/previous cameras
  (:`Pressed`
    (`self.Possess Next Camera`)))

(event `Possess Next Camera`
  ;[0.4335 1 0] Selecting next/previous cameras
  (`self.Set Camera` (+ (`self.Current Camera Index`) 1)))

(event `Possess Previous Camera`
  ;[0.4335 1 0] Selecting next/previous cameras
  (`self.Set Camera` (- (`self.Current Camera Index`) 1)))

(event `InputAction|PreviousCameraAction`
  (params (Key :type "Key Structure"))
  ;[0.4335 1 0] Selecting next/previous cameras
  (:`Pressed`
    (`self.Possess Previous Camera`)))

(event `Set Camera`
  (params (Index :type Integer))
  ;[0.2187 1 0] Setting camera
  (if (not (`self.Secondary Action`))
    (if (> (`KismetArrayLibrary.Array_Length` (`self.Cameras`)) 0)
      (set `self.Current Camera Index` (mod Index (`KismetArrayLibrary.Array_Length` (`self.Cameras`))))
      (if (!= (`|GetArrayItem` (`self.Cameras`) (`self.Current Camera Index`)) (`self.Current Camera`))
        (`|ExecutionSequence`
          (:`then_0`
            (bind _current_camera (`self.Current Camera`)
              (:`then`
                (`/ZOAN_VP/Blueprints/Camera/BP_ZVP_VirtualCamera.Set Control Enabled` _current_camera false))
              (:`else`)))
          (:`then_1`
            (bind _output_get (set `self.Current Camera` (`|GetArrayItem` (`self.Cameras`) (`self.Current Camera Index`))))
            (`/Engine/EditorBlueprintResources/StandardMacros.IsValid` _output_get
              (:`Is Valid`
                (`/ZOAN_VP/Blueprints/Camera/BP_ZVP_VirtualCamera.Set Control Enabled` _output_get true)))))
        (else
          (`KismetSystemLibrary.PrintString` "ERROR: Trying to possess the same camera" true true (struct :`R` 1.0 :`A` 1.0) 10.0)))
      (else
        (`KismetSystemLibrary.PrintString` "ERROR: Can't select camera, empty cameras array!" true true (struct :`R` 1.0 :`A` 1.0) 10.0)))))

(fn `Change Camera Group`
  (params (Direction :type "/ZOAN_VP/Blueprints/Camera/E_ZVP_CameraGroupDirection Enum" :default "NewEnumerator0"))
  (bind _returnvalue (+ (`KismetArrayLibrary.Array_Find` (`self.Active Camera Groups`) (`ZVP_Subsystem.GetCameraGroup` (subsystem `ZVP_Subsystem`))) (select `/ZOAN_VP/Blueprints/Camera/E_ZVP_CameraGroupDirection` (`local.Direction`) :`NewEnumerator0` 1 :`NewEnumerator1` -1)))
  (bind _output (`|GetArrayItem` (`self.Active Camera Groups`) (mod (select `bool` (< _returnvalue 0) :`false` _returnvalue :`true` (+ (`KismetArrayLibrary.Array_Length` (`self.Active Camera Groups`)) _returnvalue)) (`KismetArrayLibrary.Array_Length` (`self.Active Camera Groups`)))))
  (`KismetSystemLibrary.PrintString` (`|GetEnumeratorNameAsString` _output))
  (`ZVP_Subsystem.SetCameraGroup` (subsystem `ZVP_Subsystem`) _output))

(fn `Get Camera Output`
  (returns (`Camera Output` :type "MediaOutput Object Reference"))
  (bind _returnvalue (`AssetRegistry.GetAssetByObjectPath` (`AssetRegistryHelpers.GetAssetRegistry`) (`KismetStringLibrary.Conv_StringToName` (`KismetSystemLibrary.Conv_SoftObjectReferenceToString` (`.CameraOutputSoftPtr` (break `ZVP_SessionConfig` (`ZVP_Subsystem.GetSessionConfig` (subsystem `ZVP_Subsystem`)))))) false))
  (return (cast `MediaOutput` (`AssetRegistryHelpers.GetAsset` _returnvalue) :!pure true)))

(fn `Get Focus Length Scale`
  (returns (Value :type "Float (double-precision)"))
  (bind _current_camera (`self.Current Camera`)
    (:`then`
      (bind (_focal_length_range_x _focal_length_range_y) (`KismetMathLibrary.BreakVector2D` (`/ZOAN_VP/Blueprints/Camera/BP_ZVP_VirtualCamera.Focal Length Range` _current_camera)))
      (return (`KismetMathLibrary.MapRangeClamped` (`CineCameraComponent.CurrentFocalLength` (`/ZOAN_VP/Blueprints/Camera/BP_ZVP_VirtualCamera.CineCamera` _current_camera)) _focal_length_range_x _focal_length_range_y 1.0 0.1)))
    (:`else`
      (return 1.0))))

(fn `Get Keyboard Mouse Scale`
  (returns (Value :type "Float (double-precision)"))
  (return (* (`self.Current Keyboard Input Scale`) (`self.Get Focus Length Scale`))))

(fn `Sort Camera Group Array`
  (locals (i :type Integer) (Num :type Integer) (j :type Integer) (i :type Integer))
  (bind _output_get (set `local.Num` (`KismetArrayLibrary.Array_Length` (`self.Active Camera Groups`))))
  (if (< (`local.i`) _output_get) :!label _label
    (set `local.j` (- (`local.Num`) 1))
    (if (> (`local.j`) (`local.i`)) :!label _label_2
      (if (< (`|GetArrayItem` (`self.Active Camera Groups`) (`local.j`)) (`|GetArrayItem` (`self.Active Camera Groups`) (- (`local.j`) 1)))
        (`KismetArrayLibrary.Array_Swap` (`self.Active Camera Groups`) (`local.j`) (- (`local.j`) 1)))
      (set `local.j` (- (`local.j`) 1))
      (goto _label_2)
      (else
        (set `local.i` (+ (`local.i`) 1))
        (goto _label)))
    (else
      (return))))

(fn `UserConstructionScript`)