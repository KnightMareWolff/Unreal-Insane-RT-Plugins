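; Effect actor that, when triggered with string parameters, spawns a child actor component immediately or at scheduled times, or cancels pending firings on "RESET".
; Parameters become absolute times: zeros fire at once, others are chained through one timer using the gap from the previous time, so they must ascend.
; Triggers and firings print debug messages.
; The construction script labels the actor with its display name in scaled, colored text.
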(event `Reset Effect`
  ;[1 1 1] Clear everything
  (`KismetArrayLibrary.Array_Clear` (`self.Times`))
  (`KismetSystemLibrary.K2_ClearAndInvalidateTimerHandle` (`self.Current Timer Handle`)))

(event `Trigger Effect`
  (params (Parameters :type "Array of String"))
  ;[1 0.4447 0] Its default behavior is to schedule several firing events if there are parameters
  ;[1 1 1] Showing parameters
  (`KismetSystemLibrary.PrintString` (`KismetStringLibrary.Concat_StrStr` "Triggered Effect: " (`KismetSystemLibrary.GetDisplayName` self) (`KismetStringLibrary.Concat_StrStr` " [ " (`KismetStringLibrary.JoinStringArray` Parameters ", ")) " ]") true true (struct :`R` 1.0 :`G` 0.18 :`A` 1.0) 10.0)
  ;[1 1 1] Does it have time parameters?
  (if (> (`KismetArrayLibrary.Array_Length` Parameters) 0)
    ;[1 1 1] Need to reset/stop all?
    (if (`KismetStringLibrary.Contains` (`|GetArrayItem` Parameters) "RESET")
      ;[1 1 1] Clear everything
      (`self.Reset Effect`)
      (else
        ;[1 1 1] Schedule fire times
        (`KismetArrayLibrary.Array_Clear` (`self.Times`))
        (set `self.Last Time` 0.0)
        (for _array_element Parameters
          (bind _returnvalue (`KismetStringLibrary.Conv_StringToDouble` _array_element))
          (if (== _returnvalue 0.0)
            (`self.Fire Effect`)
            (else
              (`KismetArrayLibrary.Array_Add` (`self.Times`) _returnvalue))))
        (`self.Schedule Next Fire`)))
    (else
      ;[1 1 1] Just fire it
      (`self.Fire Effect`))))

(event `Schedule Next Fire`
  (bind _returnvalue (- (`|GetArrayItem` (`self.Times`)) (`self.Last Time`)))
  ;[1 1 1] Comment
  (if (> (`KismetArrayLibrary.Array_Length` (`self.Times`)) 0)
    (if (> _returnvalue 0.0)
      (bind _returnvalue_2 (`KismetSystemLibrary.K2_SetTimerDelegate` (delegate `Fire Scheduled Effect`) _returnvalue))
      (set `self.Current Timer Handle` _returnvalue_2)
      (set `self.Last Time` (`|GetArrayItem` (`self.Times`)))
      (`KismetArrayLibrary.Array_Remove` (`self.Times`))
      (else
        (`KismetSystemLibrary.PrintString` "WARNING: Got negative delay!" true true (struct :`R` 1.0 :`G` 0.466324 :`A` 1.0) 10.0)))))

(event `Fire Scheduled Effect`
  ;[1 1 1] Firing and scheduling next effect
  (`self.Fire Effect`)
  (`self.Schedule Next Fire`))

(event `Fire Effect`
  ;[1 0 0] The actual effect
  (`KismetSystemLibrary.PrintString` (`KismetStringLibrary.Concat_StrStr` "Firing Effect: " (`KismetSystemLibrary.GetDisplayName` self) (`KismetStringLibrary.Concat_StrStr` " [ " (`KismetStringLibrary.Conv_DoubleToString` (`self.Last Time`)) " ]")) true true (struct :`G` 1.0 :`B` 0.623002 :`A` 1.0) 10.0)
  (`AddComponent|NODE_AddChildActorComponent-0`))

(fn `UserConstructionScript`
  (`SceneComponent.SetRelativeScale3D` (`self.Text Root`) (`KismetMathLibrary.Conv_DoubleToVector` (`self.Title Scale`)))
  (bind _output_get (set `self.Effect Name` (`KismetSystemLibrary.GetDisplayName` self)))
  (`KismetStringLibrary.ReplaceInline` _output_get " " "_")
  (`TextRenderComponent.K2_SetText` (`self.Effect Name Text`) (`KismetTextLibrary.Conv_StringToText` (`self.Effect Name`)))
  (`TextRenderComponent.SetTextRenderColor` (`self.Effect Name Text`) (`self.Text Color`)))