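; UDP listener actor that receives network messages and rebroadcasts them through the OnUDPMessageReceived event dispatcher.
; On BeginPlay it binds connection and receive delegates on the socket client target, then starts a UDP receiver on all interfaces at ServerPort.
; StopRepeatedMessages optionally drops a message identical to the previous one.
; Connection status, received messages and skipped duplicates are printed on screen for debugging.
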(event `On Socket Connection Changed`
  (params (success :type Boolean) (message :type String) (clientConnectionID :type String))
  ;[0.447 0 1] Connection status
  (`KismetSystemLibrary.PrintString` message true true (select `bool` success :`false` (struct :`R` 1.0 :`A` 1.0) :`true` (struct :`G` 1.0 :`A` 1.0) :!type "LinearColor Structure") 10.0))

(event `self.ReceiveBeginPlay`
  (`|ExecutionSequence`
    (:`then_0`
      ;[0.447 0 1] Connection status
      (add `SocketClientBPLibrary.onsocketClientUDPConnectionEventDelegate` (`SocketClientBPLibrary.getSocketClientTarget`) (delegate `On Socket Connection Changed`)))
    (:`then_1`
      ;[1 0.008376 0] Receiving UDP messages
      (add `SocketClientBPLibrary.onreceiveUDPMessageEventDelegate` (`SocketClientBPLibrary.getSocketClientTarget`) (delegate `On Receiving UDP Message`)))
    (:`then_2`
      ;[0.4549 1 0] Initializing UDP receiver
      (`SocketClientBPLibrary.socketClientInitUDPReceiver` (`SocketClientBPLibrary.getSocketClientTarget`) "0.0.0.0" (`self.Server Port`) "E_SAB"))))

(event `On Receiving UDP Message`
  (params (message :type String) (byteArray :type "Array of Byte (by ref)") (IP_FromSender :type String) (portFromSender :type Integer) (clientConnectionID :type String))
  ;[1 0.008376 0] Receiving UDP messages
  (if (`self.Stop Repeated Messages`)
    (if (`KismetStringLibrary.NotEqual_StrStr` message (`self.Last UDP Message`))
      (set `self.Last UDP Message` message :!label _label)
      (`self.On UDP Message Received` self (`self.Last UDP Message`))
      (`KismetSystemLibrary.PrintString` (`self.Last UDP Message`) true true (struct :`G` 0.66 :`B` 1.0 :`A` 1.0) 10.0)
      (else
        (`KismetSystemLibrary.PrintString` "Got same UDP message!" true true (struct :`R` 1.0 :`B` 1.0 :`A` 1.0) 10.0)))
    (else
      (goto _label))))

(fn `UserConstructionScript`)