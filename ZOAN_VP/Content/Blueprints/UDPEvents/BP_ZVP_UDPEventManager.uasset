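; UDP event manager actor that turns incoming UDP messages into show control commands for ZVP.
; It splits each message into machine path, command and parameters, running it only when addressed to ALL or this session's machine name.
; Load opens levels and Play swaps active Level Sequences, both through data table lookups; Effect triggers matching BP_ZVP_Effect actors cached at BeginPlay.
; PANIC resets all cached effects and destroys active sequence actors.
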(event `self.ReceiveBeginPlay`
  ;[1 0 0.2948] Getting all effect actors in the scene
  (bind _outactors (`GameplayStatics.GetAllActorsOfClass` "/ZOAN_VP/Blueprints/Effects/BP_ZVP_Effect.BP_ZVP_Effect_C"))
  (set `self.Effect Actors` _outactors))

(event `Process UDP Message`
  (params (Message :type String))
  (bind _output_get (set `self.Current UDP Message` (`KismetStringLibrary.Trim` Message)))
  (bind (_lefts _rights _returnvalue) (`KismetStringLibrary.Split` _output_get " "))
  ;[0 1 0.9791] Parsing UDP message
  (set `self.Param Array` (select `bool` _returnvalue :`true` (`self.Split Parameters` _rights)))
  (bind (_lefts_2 _rights_2) (`KismetStringLibrary.Split` _lefts "/" "IgnoreCase" "FromEnd"))
  (set `self.Machine Name` _lefts_2)
  (set `self.Current Command` _rights_2)
  ;[0 0.1876 1] Is it the right machine to run this command?
  (if (`self.Can Run Command`)
    ;[0.6158 0 1] Panic command?
    (if (`KismetStringLibrary.EqualEqual_StrStr` (`self.Current Command`) "PANIC")
      ;[0.2021 1 0] Resetting everything
      (`self.Reset Everything`)
      (else
        ;[1 0.07474 0] Running event
        (`self.Run Event` (`self.Current Command`) (`self.Param Array`))))))

(event `Stop All Level Sequences`
  ;[0.5398 1 0] Stopping all active Level Sequences
  (for _array_element (`self.Active Level Sequences`)
    (`self.K2_DestroyActor` _array_element))
  (`KismetArrayLibrary.Array_Clear` (`self.Active Level Sequences`)))

(fn `Can Run Command`
  (returns (ReturnValue :type Boolean))
  (return (or (`KismetStringLibrary.Contains` (`self.Machine Name`) "ALL") (`KismetStringLibrary.Contains` (`self.Machine Name`) (`.MachineName` (break `ZVP_SessionConfig` (`ZVP_Subsystem.GetSessionConfig` (subsystem `ZVP_Subsystem`))))))))

(fn `Open Level`
  (params (`Level Name` :type String))
  ;[0.5 0 1] Opening level
  (bind _returnvalue (`|GetDataTableRow` (`self.Level Names List`) (`KismetStringLibrary.Conv_StringToName` (`local.Level Name`)))
    (:`then`
      (bind _levelname (break `/ZOAN_VP/Blueprints/UDPEvents/STR_ZVP_Event_LevelName` _returnvalue))
      (`KismetSystemLibrary.PrintString` (`KismetStringLibrary.Concat_StrStr` "Loading Level: " (`KismetStringLibrary.Conv_NameToString` _levelname)) true true (struct :`G` 0.66 :`B` 1.0 :`A` 1.0) 10.0)
      (`GameplayStatics.OpenLevel` _levelname))
    (:`RowNotFound`
      (`KismetSystemLibrary.PrintString` (`KismetStringLibrary.Concat_StrStr` "ERROR: Could not load level, no entry: " (`local.Level Name`)) true true (struct :`R` 1.0 :`A` 1.0) 10.0))))

(fn `Play Level Sequences`
  (params (`Song Name` :type String))
  ;[1 0 0.02417] Playing Level Sequence
  (bind _returnvalue (`|GetDataTableRow` (`|ConvertAsset` (`.SongsDataTableSoftPtr` (break `ZVP_ProjectConfig` (`ZVP_Subsystem.GetProjectConfig` (subsystem `ZVP_Subsystem`))))) (`KismetStringLibrary.Conv_StringToName` (`local.Song Name`)))
    (:`then`
      (`self.Stop All Level Sequences`)
      (for _array_element (`.LevelSequences_8_C94395654F4502274DF963A244117C9C` (break `/ZOAN_VP/Blueprints/UDPEvents/STR_ZVP_Event_LevelSequences` _returnvalue))
        (bind (_levelsequence _settings) (break `/ZOAN_VP/Blueprints/UDPEvents/STR_ZVP_Event_LevelSequenceConfig` _array_element))
        (`/Engine/EditorBlueprintResources/StandardMacros.IsValid` _levelsequence
          (:`Is Valid`
            (`KismetSystemLibrary.PrintString` (`KismetStringLibrary.Concat_StrStr` "Playing Level Sequence: " (`KismetSystemLibrary.GetDisplayName` _levelsequence)) true true (struct :`G` 0.66 :`B` 1.0 :`A` 1.0) 10.0)
            (bind _outactor (`LevelSequencePlayer.CreateLevelSequencePlayer` _levelsequence _settings))
            (`KismetArrayLibrary.Array_Add` (`self.Active Level Sequences`) _outactor))
          (:`Is Not Valid`
            (`KismetSystemLibrary.PrintString` (`KismetStringLibrary.Concat_StrStr` "ERROR: Could not play Level Sequence, invalid asset for: " (`local.Song Name`)))))))
    (:`RowNotFound`
      (`KismetSystemLibrary.PrintString` (`KismetStringLibrary.Concat_StrStr` "ERROR: Could not play Level Sequences, no entry: " (`local.Song Name`))))))

(fn `Reset Everything`
  (`|ExecutionSequence`
    (:`then_0`
      ;[0.5483 0 1] Resetting effects
      (for _array_element (`self.Effect Actors`)
        (`/ZOAN_VP/Blueprints/Effects/BP_ZVP_Effect.Reset Effect` _array_element)))
    (:`then_1`
      ;[1 0.3767 0] Stopping all level sequences
      (`self.Stop All Level Sequences`))))

(fn `Run Event`
  (params (Command :type String) (Parameters :type "Array of String"))
  (locals (`Effect Parameters` :type "Array of String"))
  (switch `string` Command
    (:`Load`
      ;[0.7282 0 1] Loads a new level
      (if (> (`KismetArrayLibrary.Array_Length` (`local.Parameters`)) 0)
        (`self.Open Level` (`|GetArrayItem` (`local.Parameters`)))))
    (:`Play`
      ;[1 0.5281 0] Plays a song
      (if (> (`KismetArrayLibrary.Array_Length` (`local.Parameters`)) 0)
        (`self.Play Level Sequences` (`|GetArrayItem` (`local.Parameters`)))))
    (:`Effect`
      ;[0 1 0.6552] Triggers an effect
      (if (> (`KismetArrayLibrary.Array_Length` (`local.Parameters`)) 0)
        (bind _output_get (set `local.Effect Parameters` (`local.Parameters`)))
        (`KismetArrayLibrary.Array_Remove` _output_get)
        (for _array_element (`self.Effect Actors`)
          (if (`KismetStringLibrary.EqualEqual_StrStr` (`/ZOAN_VP/Blueprints/Effects/BP_ZVP_Effect.Effect Name` _array_element) (`|GetArrayItem` (`local.Parameters`)))
            (`/ZOAN_VP/Blueprints/Effects/BP_ZVP_Effect.Trigger Effect` _array_element (`local.Effect Parameters`))))))))

(fn `Split Parameters`
  (params (Message :type String))
  (returns (Parameters :type "Array of String"))
  (locals (Params :type "Array of String") (`Left Part` :type String) (`Right Part` :type String) (`Current Message` :type String))
  (bind (_lefts _rights) (`KismetStringLibrary.Split` (`local.Current Message`) " "))
  (bind _output_get (set `local.Current Message` (`KismetStringLibrary.Trim` Message)))
  (if (`KismetStringLibrary.Contains` _output_get " ")
    (set `local.Left Part` _lefts :!label _label)
    (set `local.Right Part` _rights)
    (if (`KismetStringLibrary.NotEqual_StrStr` (`local.Current Message`) (`local.Right Part`))
      (`KismetArrayLibrary.Array_Add` (`local.Params`) (`local.Left Part`))
      (set `local.Current Message` (`local.Right Part`))
      (goto _label)
      (else
        (`KismetArrayLibrary.Array_Add` (`local.Params`) (`local.Right Part`))
        (return (`local.Params`))))
    (else
      (`KismetArrayLibrary.Array_Add` (`local.Params`) (`local.Current Message`))
      (return (`local.Params`)))))

(fn `UserConstructionScript`)