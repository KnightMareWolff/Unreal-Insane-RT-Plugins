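; Virtual production manager actor that bootstraps the ZVP runtime on BeginPlay and enables SteamVR input via console command.
; It finds or spawns the camera manager, UDP event manager and UDP listener, and shows an optional startup widget.
; Event manager and listener classes come from the ZVP project config with default fallbacks, as does the listener's port.
; Received UDP messages are forwarded to the event manager for processing.
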(event `self.ReceiveBeginPlay`
  (`KismetSystemLibrary.ExecuteConsoleCommand` "vr.SteamVR.EnableVRInput 1" (`GameplayStatics.GetPlayerController` 0))
  (`|ExecutionSequence`
    (:`then_0`
      ;[0 0.5216 1] Checking existing camera manager
      (bind _returnvalue (`GameplayStatics.GetActorOfClass` "/ZOAN_VP/Blueprints/Camera/BP_ZVP_CameraManager.BP_ZVP_CameraManager_C"))
      (`/Engine/EditorBlueprintResources/StandardMacros.IsValid` _returnvalue
        (:`Is Valid`
          ;[0.9942 0.1214 1] Simple assigning existing camera manager
          (set `self.VP Camera Manager` _returnvalue))
        (:`Is Not Valid`
          ;[0 0.6719 1] Spawning camera manager
          (bind _returnvalue_2 (`|SpawnActorFromClass` "/ZOAN_VP/Blueprints/Camera/BP_ZVP_CameraManager.BP_ZVP_CameraManager_C" (`KismetMathLibrary.MakeTransform` (0.0 0.0 0.0)) "AlwaysSpawn" "OverrideRootScale" null null))
          (set `self.VP Camera Manager` _returnvalue_2))))
    (:`then_1`
      ;[0.3785 0.1247 1] Startup widget
      (`self.Spawn Startup Widget`))
    (:`then_2`
      ;[0.1988 0 1] Dealing with UDP Event Manager
      (bind _returnvalue_3 (`GameplayStatics.GetActorOfClass` "/ZOAN_VP/Blueprints/UDPEvents/BP_ZVP_UDPEventManager.BP_ZVP_UDPEventManager_C"))
      (`/Engine/EditorBlueprintResources/StandardMacros.IsValid` _returnvalue_3
        (:`Is Valid`
          (set `self.UDP Event Manager` _returnvalue_3))
        (:`Is Not Valid`
          (bind _returnvalue_4 (`|SpawnActorFromClass` (`self.Get Event Manager Class`) (`KismetMathLibrary.MakeTransform` (0.0 0.0 0.0)) "AlwaysSpawn" "OverrideRootScale" null null))
          (set `self.UDP Event Manager` _returnvalue_4))))
    (:`then_3`
      ;[1 0.07017 0] Dealing with UDP Server
      (bind _returnvalue_5 (`GameplayStatics.GetActorOfClass` "/ZOAN_VP/Blueprints/UDPEvents/BP_ZVP_UDPListener.BP_ZVP_UDPListener_C"))
      (`/Engine/EditorBlueprintResources/StandardMacros.IsValid` _returnvalue_5
        (:`Is Valid`
          (set `self.UDP Listener` _returnvalue_5))
        (:`Is Not Valid`
          (bind _returnvalue_6 (`|SpawnActorFromClass` (`self.Get Event Listener Class`) (`KismetMathLibrary.MakeTransform` (0.0 0.0 0.0)) "AlwaysSpawn" "OverrideRootScale" null (`.UDPPort` (break `ZVP_ProjectConfig` (`ZVP_Subsystem.GetProjectConfig` (subsystem `ZVP_Subsystem`)))) null))
          (set `self.UDP Listener` _returnvalue_6)))
      ;[0 1 0.4243] Sending UDP message to Event manager
      (add `/ZOAN_VP/Blueprints/UDPEvents/BP_ZVP_UDPListener.On UDP Message Received` (`self.UDP Listener`) (delegate `On UDP Message Received`)))))

(event `On UDP Message Received`
  (params (`UDP Listener` :type "/ZOAN_VP/Blueprints/UDPEvents/BP_ZVP_UDPListener Object Reference") (Message :type String))
  ;[0 1 0.4243] Sending UDP message to Event manager
  (`/ZOAN_VP/Blueprints/UDPEvents/BP_ZVP_UDPEventManager.Process UDP Message` (`self.UDP Event Manager`) Message))

(event `Spawn Startup Widget`
  ;[1 0.4333 0] Spawining startup widget screen
  (bind _startup_widget_class (`self.Startup Widget Class`)
    (:`then`
      (bind _returnvalue (`|CreateWidget` _startup_widget_class (`GameplayStatics.GetPlayerController` 0)))
      (bind _output_get (set `self.Startup Widget` _returnvalue))
      (`UserWidget.AddToViewport` _output_get 0)
      (add `/ZOAN_VP/Blueprints/UI/UI_ZVP_StartupScreen.On Done` _output_get (delegate `Startup Widget Done`)))
    (:`else`)))

(event `Startup Widget Done`
  ;[1 0.4333 0] Spawining startup widget screen
)

(fn `Get Event Listener Class`
  (returns (`UDP Listener Class` :type "/ZOAN_VP/Blueprints/UDPEvents/BP_ZVP_UDPListener Class Reference"))
  (bind (_asbp_zvp_udplistener _bsuccess) (castclass `/ZOAN_VP/Blueprints/UDPEvents/BP_ZVP_UDPListener` (`|ConvertAsset` (`.EventListenerClassSoftPtr` (break `ZVP_ProjectConfig` (`ZVP_Subsystem.GetProjectConfig` (subsystem `ZVP_Subsystem`))))) :!pure true))
  (return (select `bool` _bsuccess :`false` (`self.Default UDP Listener Class`) :`true` _asbp_zvp_udplistener)))

(fn `Get Event Manager Class`
  (returns (`Event Manager Class` :type "/ZOAN_VP/Blueprints/UDPEvents/BP_ZVP_UDPEventManager Class Reference"))
  (bind (_asbp_zvp_udpevent_manager _bsuccess) (castclass `/ZOAN_VP/Blueprints/UDPEvents/BP_ZVP_UDPEventManager` (`|ConvertAsset` (`.EventManagerClassSoftPtr` (break `ZVP_ProjectConfig` (`ZVP_Subsystem.GetProjectConfig` (subsystem `ZVP_Subsystem`))))) :!pure true))
  (return (select `bool` _bsuccess :`false` (`self.Default UDP Event Manager Class`) :`true` _asbp_zvp_udpevent_manager)))

(fn `UserConstructionScript`)