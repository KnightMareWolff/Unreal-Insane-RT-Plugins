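; BP_ZVP_Screen is a screen actor whose plane shows or hides according to the real camera type.
; Virtual and On Rails types open the media source and reveal the screen; Handheld closes the source and hides it.
; BeginPlay attaches the plane to a pivot component to simplify an aim-to-camera feature.
; Initial setup and camera-change listening in this Blueprint are unused, having moved to the Camera Manager.
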(event `self.ReceiveBeginPlay`
  (`parent.ReceiveBeginPlay`)
  (`SceneComponent.K2_AttachToComponent` (`self.Plane`) (`self.Plane Pivot`) "None" "KeepWorld" "KeepWorld" "KeepWorld" true) ; Using a pivot component to make aim to camera feature easier to code
)

(event `Adapt Camera Type`
  (params (CameraType :type "EZVP_CameraType Enum" :default "ZVP_Virtual"))
  ;[0.08961 1 0] Adapting screen to real camera type
  (switch `EZVP_CameraType` CameraType
    (:`ZVP_Virtual`
      (`self.RequestOpenMediaSource` :!label _label)
      (`SceneComponent.SetVisibility` (`self.RootComponent`) true true))
    (:`ZVP_Handheld`
      (`self.RequestCloseMediaSource`)
      (`SceneComponent.SetVisibility` (`self.RootComponent`) false true))
    (:`ZVP_OnRails`
      (goto _label))))

(fn `UserConstructionScript`
  (`parent.UserConstructionScript`))